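; Mod actor for AdvancedShortcuts that adds keyboard shortcuts for opening game HUD panels such as agent manager, stockpile, debt, quests, policies and tech tree.
; On BeginPlay it enables input from player one.
; Ctrl or Shift plus number keys cast to PlayerController_Play and send named HUD actions through HandleHudAction, including idler selection.
; The 0 key logs every user widget's name and path through the mod API, apparently for debugging.
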(event EventBeginPlay
  (Input|EnableInput (Game|GetPlayerController 0)))

(event Collision|EventActorBeginOverlap
  (params (OtherActor :type Actor%20Object%20Reference)))

(event EventTick
  (params (DeltaSeconds :type Float%20%28single-precision%29)))

(event Input|KeyboardEvents|0
  (params (Key :type Key%20Structure :default "None"))
  (:Pressed
    (bind _foundwidgets (Widget|GetAllWidgetsOfClass "/Script/UMG.UserWidget" false))
    (for _array_element _foundwidgets
      (Class|ModAPI|LogMessage (Class|ModAPI|GetModAPI) (Utilities|String|Append (Utilities|GetDisplayName _array_element) ": " (Class|KismetSystemLibrary|GetPathName _array_element)) false))))

(event Input|KeyboardEvents|Shift7
  (params (Key :type Key%20Structure :default "None"))
  (:Pressed
    (bind _asplayer_controller_play (Utilities|Casting|CastToPlayerController_Play (Game|GetPlayerController 0)))
    (Class|PlayerControllerPlay|HandleHudAction _asplayer_controller_play (Utilities|Struct|MakeHudAction "openTechTree"))))

(event Input|KeyboardEvents|Shift1
  (params (Key :type Key%20Structure :default "None"))
  (:Pressed
    (bind _asplayer_controller_play (Utilities|Casting|CastToPlayerController_Play (Game|GetPlayerController 0)))
    (Class|PlayerControllerPlay|HandleHudAction _asplayer_controller_play (Utilities|Struct|MakeHudAction "agentmenu"))))

(event Input|KeyboardEvents|Shift2
  (params (Key :type Key%20Structure :default "None"))
  (:Pressed
    (bind _asplayer_controller_play (Utilities|Casting|CastToPlayerController_Play (Game|GetPlayerController 0)))
    (Class|PlayerControllerPlay|HandleHudAction _asplayer_controller_play (Utilities|Struct|MakeHudAction "stockpileview"))))

(event Input|KeyboardEvents|Shift3
  (params (Key :type Key%20Structure :default "None"))
  (:Pressed
    (bind _asplayer_controller_play (Utilities|Casting|CastToPlayerController_Play (Game|GetPlayerController 0)))
    (Class|PlayerControllerPlay|HandleHudAction _asplayer_controller_play (Utilities|Struct|MakeHudAction "openDebtView"))))

(event Input|KeyboardEvents|Shift6
  (params (Key :type Key%20Structure :default "None"))
  (:Pressed
    (bind _asplayer_controller_play (Utilities|Casting|CastToPlayerController_Play (Game|GetPlayerController 0)))
    (Class|PlayerControllerPlay|HandleHudAction _asplayer_controller_play (Utilities|Struct|MakeHudAction "openProductionLimitControls"))))

(event Input|KeyboardEvents|Shift4
  (params (Key :type Key%20Structure :default "None"))
  (:Pressed
    (bind _asplayer_controller_play (Utilities|Casting|CastToPlayerController_Play (Game|GetPlayerController 0)))
    (Class|PlayerControllerPlay|HandleHudAction _asplayer_controller_play (Utilities|Struct|MakeHudAction "openQuestLog"))))

(event Input|KeyboardEvents|Shift5
  (params (Key :type Key%20Structure :default "None"))
  (:Pressed
    (bind _asplayer_controller_play (Utilities|Casting|CastToPlayerController_Play (Game|GetPlayerController 0)))
    (Class|PlayerControllerPlay|HandleHudAction _asplayer_controller_play (Utilities|Struct|MakeHudAction "openPolicyView"))))

(event Input|KeyboardEvents|Ctrl1
  (params (Key :type Key%20Structure :default "None"))
  (:Pressed
    (bind _asplayer_controller_play (Utilities|Casting|CastToPlayerController_Play (Game|GetPlayerController 0)))
    (Class|PlayerControllerPlay|HandleHudAction _asplayer_controller_play (Utilities|Struct|MakeHudAction "openAgentManager"))))

(event Input|KeyboardEvents|Ctrl2
  (params (Key :type Key%20Structure :default "None"))
  (:Pressed
    (bind _asplayer_controller_play (Utilities|Casting|CastToPlayerController_Play (Game|GetPlayerController 0)))
    (Class|PlayerControllerPlay|HandleHudAction _asplayer_controller_play (Utilities|Struct|MakeHudAction "selectIdler"))))

(fn ConstructionScript)